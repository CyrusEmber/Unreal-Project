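; BP_BinggyCharacter is a character Blueprint that drives the player's overhead name display and health bar widgets.
; On BeginPlay it has the overhead widget show the player's name, then binds to the HealthComponent's health and max health change events.
; Either event refreshes the overhead health bar with the component's normalized health.
; The binding only runs if the overhead widget cast succeeds.
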(event `self.ReceiveBeginPlay`
  ;[1 1 1] Create Overhead widget
  (bind _aswbp_over_head_widget (cast `/Game/Blueprints/UI/WBP_OverHeadWidget` (`WidgetComponent.GetUserWidgetObject` (`self.OverheadWidget`))))
  (`OverHeadWidget.ShowPlayerName` _aswbp_over_head_widget self)
  ;[1 1 1] Health Bar Binding, it only bind to the overhead health bar
  (`|ExecutionSequence`
    (:`then_0`
      (add `BinggyHealthComponent.OnHealthChanged` (`self.HealthComponent`) (delegate `OnHealthChanged_Event`)))
    (:`then_1`
      (add `BinggyHealthComponent.OnMaxHealthChanged` (`self.HealthComponent`) (delegate `OnMaxHealthChanged_Event`)))))

(event `OnHealthChanged_Event`
  (params (NewValue :type "Float (single-precision)"))
  ;[1 1 1] Health Bar Binding, it only bind to the overhead health bar
  (`self.SetHealthBarPercent`))

(event `OnMaxHealthChanged_Event`
  (params (NewValue :type "Float (single-precision)"))
  ;[1 1 1] Health Bar Binding, it only bind to the overhead health bar
  (`self.SetHealthBarPercent`))

(fn `SetHealthBarPercent`
  (bind _aswbp_progress_bar_base (cast `/Game/Blueprints/UI/ProgressBar/WBP_ProgressBarBase` (`WidgetComponent.GetUserWidgetObject` (`self.HealthBar`))))
  (`/Game/Blueprints/UI/ProgressBar/WBP_ProgressBarBase.SetBarPercentage` _aswbp_progress_bar_base (`BinggyHealthComponent.GetHealthNormalized` (`self.HealthComponent`))))

(fn `UserConstructionScript`)