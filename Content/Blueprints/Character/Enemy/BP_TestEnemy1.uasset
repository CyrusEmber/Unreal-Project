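; BP_TestEnemy1 is a test enemy Blueprint with a HealthComponent and a HealthBar widget.
; BeginPlay binds handlers to the component's health and max-health change events, but both handlers are empty.
; SetHealthBarPercent pushes normalized health into the WBP_ProgressBarBase widget, but its two calls in the event graph are disconnected, so this Blueprint never updates the bar.
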(event `self.ReceiveBeginPlay`
  (`|ExecutionSequence`
    (:`then_0`
      (add `BinggyHealthComponent.OnHealthChanged` (`self.HealthComponent`) (delegate `OnHealthChanged_Event`)))
    (:`then_1`
      (add `BinggyHealthComponent.OnMaxHealthChanged` (`self.HealthComponent`) (delegate `OnMaxHealthChanged_Event`)))))

(event `OnHealthChanged_Event`
  (params (NewValue :type "Float (single-precision)")))

(event `OnMaxHealthChanged_Event`
  (params (NewValue :type "Float (single-precision)")))

(fn `SetHealthBarPercent`
  (bind _aswbp_progress_bar_base (cast `/Game/UI/UserWidget/ProgressBar/WBP_ProgressBarBase` (`WidgetComponent.GetUserWidgetObject` (`self.HealthBar`))))
  (`/Game/UI/UserWidget/ProgressBar/WBP_ProgressBarBase.SetBarPercentage` _aswbp_progress_bar_base (`BinggyHealthComponent.GetHealthNormalized` (`self.HealthComponent`))))

(fn `UserConstructionScript`)