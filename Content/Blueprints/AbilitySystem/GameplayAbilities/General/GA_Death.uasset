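; GA_Death is a general death gameplay ability that tells the avatar to die.
; When activated from an event, it calls Die through the avatar's CombatInterface, passing the impulse direction and hit bone name from the event's effect context.
; The ability never calls EndAbility in this graph.
; Its RagDoll function is empty, with disconnected leftover nodes for physics simulation and a velocity-based impulse that never run.
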(event `self.K2_ActivateAbility`)

(event `self.K2_ActivateAbilityFromEvent`
  (params (EventData :type "GameplayEventData Structure (by ref)"))
  (bind (_eventtag _instigator _target _optionalobject _optionalobject2 _contexthandle) (break `GameplayEventData` EventData))
  (bind _ascombat_interface (cast `CombatInterface` (`self.GetAvatarActorFromActorInfo`)))
  (`CombatInterface.Die` _ascombat_interface (`UtilityLibrary.GetImpulseDirection` _contexthandle) (`.HitBoneName` (`GameplayStatics.BreakHitResult` (`AbilitySystemBlueprintLibrary.EffectContextGetHitResult` _contexthandle)))))

(fn `RagDoll`
  ;[1 1 1] Activate Character Physics
)