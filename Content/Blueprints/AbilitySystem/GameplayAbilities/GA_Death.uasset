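; GA_Death is a gameplay ability that triggers death on its avatar actor.
; On activation it casts the avatar to CombatInterface, calls Die and prints a debug "Death" string, without calling EndAbility.
; An Elimination call on BinggyCharacter is left unconnected.
; The RagDoll function is an empty stub, with disconnected nodes for ragdoll collision, bone physics simulation and a velocity-based impulse.
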(event `self.K2_ActivateAbility`
  (bind _ascombat_interface (cast `CombatInterface` (`self.GetAvatarActorFromActorInfo`)))
  (`CombatInterface.Die` _ascombat_interface)
  (`KismetSystemLibrary.PrintString` "Death"))

(fn `RagDoll`
  ;[1 1 1] Activate Character Physics
)